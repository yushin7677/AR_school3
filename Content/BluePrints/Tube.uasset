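; Tube Blueprint that sets up temperature-related visual data for its STANDTUBE component, all on BeginPlay.
; It bakes Data Table rows into the ShitRT render target as a color strip, one canvas line per row, using Con's Y, Z and W as RGB.
; It then calls TempUpdate, packs FullTemp into Custom Primitive Data as four vectors, and slightly lowers MaxTemp once.
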(event EventBeginPlay
  (bind _fulltemp (Variables|Default|GetfullTemp))
  (bind _datatable (Variables|Default|GetDataTable))
  (bind _shitrt (Variables|Default|GetShitRT))
  (Rendering|ClearRenderTarget2D _shitrt)
  (bind (_canvas _size _context) (Rendering|BeginDrawCanvastoRenderTarget _shitrt))
  (bind _outrownames (DataTable|GetDataTableRowNames _datatable))
  (for (_array_element _array_index) _outrownames
    (bind _returnvalue (Utilities|GetDataTableRow _datatable _array_element)
      (:then
        (Class|Canvas|DrawLine _canvas (Math|Vector2D|MakeVector2D (Math|Conversions|ToFloat(Integer) _array_index) 0.0) (Math|Vector2D|MakeVector2D (+ (Math|Conversions|ToFloat(Integer) _array_index) 1.0) 0.0) 1e+01 (Utilities|Struct|MakeLinearColor (.y (Utilities|Struct|Break4vector _returnvalue)) (.z (Utilities|Struct|Break4vector _returnvalue)) (.w (Utilities|Struct|Break4vector _returnvalue)) 1.0)))))
  (Rendering|EndDrawCanvastoRenderTarget _context)
  (Class|ThBody|TempUpdate 25.0 (Variables|Default|GetmaxTemp))
  (for _index (range 0 3)
    (Rendering|Material|SetCustomPrimitiveDataVector3 (Variables|Default|GetSTAND_TUBE) (* _index 3) (Math|Vector|MakeVector (Utilities|Array|Get(acopy) _fulltemp (+ (* _index 3) 0)) (Utilities|Array|Get(acopy) _fulltemp (+ (* _index 3) 1)) (Utilities|Array|Get(acopy) _fulltemp (+ (* _index 3) 2)))))
  (Variables|Default|SetmaxTemp (- (Variables|Default|GetmaxTemp) 0.1)))

(fn ConstructionScript)