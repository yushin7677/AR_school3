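; AR pawn that lets the player place a stand and a tube on a detected real-world surface.
; It starts an AR session on BeginPlay and debug-draws all tracked geometry each tick until placement.
; A touch press line-traces from the finger's screen position, ignoring feature points, and spawns both actors at the first hit.
; The HaveStand flag then stops both the drawing and further placement.
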(event EventBeginPlay
  (Class|ARBlueprintLibrary|StartARSession "/Game/BluePrints/AR1.AR1"))

(event EventTick
  (params (DeltaSeconds :type Float%20%28single-precision%29))
  (if (not (Variables|Default|Gethave%20stand))
    ;[1 1 1] Прорисовка всех видимых планов
    (bind _returnvalue (Class|ARBlueprintLibrary|GetAllGeometries))
    (bind _array_element (Utilities|Array|ForEachLoopwithBreak _returnvalue)
      (:LoopBody
        (Class|ARBlueprintLibrary|DebugDrawTrackedGeometry _array_element "(R=1.000000,G=0.635500,B=0.000000,A=1.000000)")))))

(event Input|TouchEvents|Touch1
  (params (Key :type Key%20Structure :default "None"))
  (bind _returnvalue (Game|GetPlayerController 0))
  (bind (_locationx _locationy) (Class|PlayerController|GetInputTouchState _returnvalue "Touch1"))
  (:Pressed
    (if (not (Variables|Default|Gethave%20stand))
      ;[0.09412 1 0] Если луч пересекает планы, то возвращается координата первого пересечения, а в этом месте спаунится стенд и труба с переменным материалом
      (bind _returnvalue_2 (Class|ARBlueprintLibrary|LineTraceTrackedObjects (Math|Vector2D|MakeVector2D _locationx _locationy) false))
      (Math|Integer|CompareInt (Utilities|Array|Length _returnvalue_2)
        (:>
          (Game|SpawnActorfromClass "/Game/BluePrints/Stand.Stand_C" (Math|Transform|MakeTransform (.location (Class|ARTraceResultLibrary|GetLocaltoWorldTransform (Utilities|Array|Get(acopy) _returnvalue_2))) "0, 0, 0" "1,1,1") "Undefined" 0 0)
          (Game|SpawnActorfromClass "/Game/BluePrints/Tube.Tube_C" (Math|Transform|MakeTransform (.location (Class|ARTraceResultLibrary|GetLocaltoWorldTransform (Utilities|Array|Get(acopy) _returnvalue_2))) "0, 0, 0" "1,1,1") "Undefined" 0 0)
          (Variables|Default|Sethave%20stand true))))))

(fn ConstructionScript)